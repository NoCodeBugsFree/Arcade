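; Arcade HUD Blueprint with helpers to draw health icons, a points readout and a clickable pause icon from game mode data.
; Helpers scale coordinates by viewport scale and offset them by screen anchors.
; BeginPlay, DrawHUD and HitBoxClick are empty; their game mode binding, draw calls and pause-menu logic sit disconnected.
; OnGameOver adds a game-over widget, but its binding never runs.
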(event `self.ReceiveBeginPlay`
  ;[0 0.1105 0.5] EBP Set GM Reference
)

(event `OnGameOver`
  ;[0 0.1105 0.5] EBP Set GM Reference
  (bind _returnvalue (`|CreateWidget` "/Game/BP/UMG/WBP_GameOver.WBP_GameOver_C"))
  (`UserWidget.AddToViewport` _returnvalue 0))

(event `self.ReceiveDrawHUD`
  (params (SizeX :type Integer) (SizeY :type Integer))
  ;[0 0.1105 0.5] Draw HUD
)

(event `self.ReceiveHitBoxClick`
  (params (BoxName :type Name))
  ;[0 0.1105 0.5] Hit Box Clicked
)

(fn `ApplyCordsAncorsBP`
  (params (In :type "Vector2D Structure") (Anchor :type "Vector2D Structure"))
  (returns (Out :type "Vector2D Structure"))
  ;[0 0.1105 0.5] Comment
  (return (+ In (* Anchor (`WidgetLayoutLibrary.GetViewportSize`)))))

(fn `DrawHealthBP`
  (bind (_out_x _out_y) (`KismetMathLibrary.BreakVector2D` (`self.ScaleCordsBP` (64.0 64.0))))
  ;[0 0.1105 0.5] Comment
  (for _index (range (`GameHealthComponent.Healths` (`ArcadeGameModeBase.GameHealthComponent` (`self.GM_BP`))))
    (bind (_out_x_2 _out_y_2) (`KismetMathLibrary.BreakVector2D` (`self.ScaleCordsBP` (`KismetMathLibrary.MakeVector2D` (+ (* _index (+ 64.0 10.0)) 20.0) 20.0))))
    (`self.DrawTexture` "/Engine/EngineResources/AICON-Green.AICON-Green" _out_x_2 _out_y_2 _out_x _out_y 0.0 0.0 1.0 1.0 (struct :`R` 1.0 :`G` 1.0 :`B` 1.0 :`A` 1.0) "BLEND_Masked")))

(fn `DrawPauseBP`
  (bind (_out_x _out_y) (`KismetMathLibrary.BreakVector2D` (`self.ScaleCordsBP` (64.0 64.0))))
  (bind (_out_x_2 _out_y_2) (`KismetMathLibrary.BreakVector2D` (`self.ApplyCordsAncorsBP` (`self.ScaleCordsBP` (-84.0 20.0)) (1.0 0.0))))
  ;[0 0.1105 0.5] Comment
  (`self.DrawTexture` "/Engine/EditorResources/Ai_Spawnpoint.Ai_Spawnpoint" _out_x_2 _out_y_2 _out_x _out_y 0.0 0.0 1.0 1.0)
  (`self.AddHitBox` (`self.ApplyCordsAncorsBP` (`self.ScaleCordsBP` (-84.0 20.0)) (1.0 0.0)) (`self.ScaleCordsBP` (64.0 64.0)) "Pause"))

(fn `DrawPointsBp`
  (bind _returnvalue (`KismetStringLibrary.Conv_IntToString` (`ArcadeGameModeBase.GamePoints` (`self.GM_BP`))))
  (bind (_out_x _out_y) (`KismetMathLibrary.BreakVector2D` (`self.ApplyCordsAncorsBP` (`self.ScaleCordsBP` (`KismetMathLibrary.MakeVector2D` (/ (`self.GetTextSize` _returnvalue "/Game/BP/UMG/Fonts/ArcadeFont.ArcadeFont") -1.0) 20.0)) (0.5 0.0))))
  ;[0 0.1105 0.5] Comment
  (`self.DrawText` (`KismetStringLibrary.Concat_StrStr` "Points: " _returnvalue) (struct :`R` 1.0 :`G` 0.283963 :`A` 0.8) _out_x _out_y "/Game/BP/UMG/Fonts/ArcadeFont.ArcadeFont"))

(fn `ScaleCordsBP`
  (params (In :type "Vector2D Structure"))
  (returns (Out :type "Vector2D Structure"))
  ;[0 0.1105 0.5] Comment
  (return (* In (`WidgetLayoutLibrary.GetViewportScale`))))

(fn `UserConstructionScript`)